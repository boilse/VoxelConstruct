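; Player controller for sculpting voxel terrain, placing Stone or carving Air with a spherical brush of adjustable radius.
; Enhanced Input triggers edits on press and periodically while held, with a debug sphere previewing the camera-ray target.
; ModifyGridSphere requires a chunk hit, edits that chunk, then propagates to other chunks found by sphere overlap.
; Hits are nudged inward against rounding; placement uses the ray's end unless the hit lies near it.
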(event `self.ReceiveTick`
  (params (DeltaSeconds :type "Float (single-precision)"))
  (bind _playercameramanager (`self.PlayerCameraManager`))
  (bind (_returnvalue _outhit) (`self.RayCast`))
  (bind (_bblockinghit _binitialoverlap _time _distance _location _impactpoint _normal) (`GameplayStatics.BreakHitResult` _outhit))
  (`KismetSystemLibrary.DrawDebugSphere` (`KismetMathLibrary.SelectVector` (- _location _normal) (+ (`PlayerCameraManager.GetCameraLocation` _playercameramanager) (* (`KismetMathLibrary.GetForwardVector` (`PlayerCameraManager.GetCameraRotation` _playercameramanager)) (`self.BlockDistance`))) _returnvalue) (`KismetMathLibrary.Conv_IntToDouble` (* (`self.Radius`) 10)) 12 (struct :`R` 1.0 :`G` 1.0 :`B` 1.0 :`A` 1.0) 0.0 1.0))

(event `self.ReceiveBeginPlay`
  (bind _returnvalue (subsystem `EnhancedInputLocalPlayerSubsystem`))
  (`/Engine/EditorBlueprintResources/StandardMacros.IsValid` _returnvalue
    (:`Is Valid`
      (`EnhancedInputSubsystemInterface.AddMappingContext` _returnvalue "/VoxelConstruct/Blueprints/Input/IMC_VoxelConstructInput.IMC_VoxelConstructInput" 0 (struct)))))

(event `EnhancedInput|/VoxelConstruct/Blueprints/Input/IA_PlaceBlock`
  (params (ActionValue :type Boolean) (ElapsedSeconds :type "Float (double-precision)") (TriggeredSeconds :type "Float (double-precision)") (InputAction :type "InputAction Object Reference" :default "/VoxelConstruct/Blueprints/Input/IA_PlaceBlock.IA_PlaceBlock"))
  ;[1 1 1] Destroy Blocks
  (:`Triggered`
    (if (`KismetMathLibrary.NearlyEqual_FloatFloat` (mod TriggeredSeconds 0.1) 0.0 0.01)
      (`self.ModifyGridSphere` "Stone" true :!label _label)))
  (:`Started`
    (goto _label)))

(event `Key|LeftMouseButton`
  (params (Key :type "Key Structure"))
  ;[1 1 1] Remove Voxel
)

(event `EnhancedInput|/VoxelConstruct/Blueprints/Input/IA_DestroyBlock`
  (params (ActionValue :type Boolean) (ElapsedSeconds :type "Float (double-precision)") (TriggeredSeconds :type "Float (double-precision)") (InputAction :type "InputAction Object Reference" :default "/VoxelConstruct/Blueprints/Input/IA_DestroyBlock.IA_DestroyBlock"))
  ;[1 1 1] Destroy Blocks
  (:`Triggered`
    (if (`KismetMathLibrary.NearlyEqual_FloatFloat` (mod TriggeredSeconds 0.1) 0.0 0.01)
      (`self.ModifyGridSphere` "Air" :!label _label_2)))
  (:`Started`
    (goto _label_2)))

(event `EnhancedInput|/VoxelConstruct/Blueprints/Input/IA_ChangeRadius`
  (params (ActionValue :type "Float (double-precision)") (ElapsedSeconds :type "Float (double-precision)") (TriggeredSeconds :type "Float (double-precision)") (InputAction :type "InputAction Object Reference" :default "/VoxelConstruct/Blueprints/Input/IA_ChangeRadius.IA_ChangeRadius"))
  (:`Triggered`
    (set `self.Radius` (`KismetMathLibrary.Clamp` (`KismetMathLibrary.FTrunc` (+ (`self.Radius`) ActionValue)) 1 10))))

(fn `ModifyGridSphere`
  (params (Block :type "EBlockType Enum" :default "Null") (Close :type Boolean))
  (bind _playercameramanager (`self.PlayerCameraManager`))
  (bind (_returnvalue _outhit _returnvalue1) (`self.RayCast`))
  (bind (_bblockinghit _binitialoverlap _time _distance _location _impactpoint _normal _impactnormal _physmat _hitactor) (`GameplayStatics.BreakHitResult` _outhit))
  (bind _asvoxel_construct_chunk_base (cast `VoxelConstructChunkBase` _hitactor))
  (bind _returnvalue_2 (`KismetMathLibrary.SelectVector` (- _location _normal) (+ (`PlayerCameraManager.GetCameraLocation` _playercameramanager) (* (`KismetMathLibrary.GetForwardVector` (`PlayerCameraManager.GetCameraRotation` _playercameramanager)) (`self.BlockDistance`))) _returnvalue))
  (bind _returnvalue_3 (select `bool` Close :`false` _returnvalue_2 :`true` (select `bool` (< (`KismetMathLibrary.Vector_Distance` _returnvalue1 _returnvalue_2) 150.0) :`false` _returnvalue1 :`true` _returnvalue_2)))
  (bind _blockscale (`VoxelConstructChunkBase.BlockScale` _asvoxel_construct_chunk_base))
  (bind _returnvalue_4 (`KismetMathLibrary.FTruncVector` (/ _returnvalue_3 _blockscale)))
  (`VoxelConstructChunkBase.ModifyVoxelBySphere` _asvoxel_construct_chunk_base _returnvalue_4 (`self.Radius`) (cast `EBlockType` Block))
  (bind _outactors (`KismetSystemLibrary.SphereOverlapActors` _returnvalue_3 (* (`self.Radius`) _blockscale) (`|MakeArray` "ObjectTypeQuery1" "ObjectTypeQuery2" :!type "EObjectTypeQuery Enum") "/Script/VoxelConstruct.VoxelConstructChunkBase"))
  (for _array_element _outactors
    (if (!= _array_element _hitactor)
      (bind _asvoxel_construct_chunk_base_2 (cast `VoxelConstructChunkBase` _array_element))
      (`VoxelConstructChunkBase.ModifyVoxelBySphere` _asvoxel_construct_chunk_base_2 _returnvalue_4 (`self.Radius`) (cast `EBlockType` Block)))))

(fn `RayCast`
  (returns (ReturnValue :type Boolean) (OutHit :type "HitResult Structure") (ReturnValue1 :type "Vector Structure"))
  (bind _playercameramanager (`self.PlayerCameraManager`))
  (bind _returnvalue (`PlayerCameraManager.GetCameraLocation` _playercameramanager))
  (bind _returnvalue_2 (+ _returnvalue (* (`KismetMathLibrary.GetForwardVector` (`PlayerCameraManager.GetCameraRotation` _playercameramanager)) (`self.BlockDistance`))))
  (bind (_outhit _returnvalue_3) (`KismetSystemLibrary.LineTraceSingle` :`Start` _returnvalue :`End` _returnvalue_2 :`TraceChannel` "TraceTypeQuery1" :`DrawTime` 10.0))
  (return _returnvalue_3 _outhit _returnvalue_2))

(fn `UserConstructionScript`)